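; BP_SubGoalJournal is a journal that shows quest sub-goals through a W_SubGoalJournal widget on its widget component.
; On BeginPlay it loops over its Quests and each quest's SubGoals, creating a W_SubGoals entry per goal inside the journal's SubGoals container.
; The same inner loop sets CanTeleport to false on the player's MotionControllerPawn.
; FillJournal is an empty stub, and a debug string prints for each quest.
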(event Custom|FillJournal)

(event EventBeginPlay
  (bind _asw_sub_goal_journal (Utilities|Casting|CastTow_SubGoalJournal (UserInterface|GetUserWidgetObject (Variables|Default|GetWidget))))
  (for _array_element (Variables|Default|GetQuests)
    (Development|PrintString "квест")
    (for _array_element_2 (.SubGoals (Utilities|Struct|Breaks_QuestInfo (Variables|/Game/Blueprints/Quests/BP_MasterQuest.BP_MasterQuest_C|GetQuestInfo _array_element)))
      (bind _returnvalue (UserInterface|CreateWidget "/Game/Widgets/w_SubGoals.w_SubGoals_C" (Game|GetPlayerController 0) _array_element_2))
      (Widget|Panel|AddChild (Variables|/Game/Widgets/w_SubGoalJournal.w_SubGoalJournal_C|GetSubGoals _asw_sub_goal_journal) _returnvalue)
      (bind _asmotion_controller_pawn (Utilities|Casting|CastToMotionControllerPawn (Game|Player|GetPlayerPawn 0)))
      (Variables|/Game/VirtualRealityBP/Blueprints/MotionControllerPawn.MotionControllerPawn_C|SetCanTeleport? _asmotion_controller_pawn false))))

(fn ConstructionScript)