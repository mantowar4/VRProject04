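; BP_GoalsInteractMaster is an interactable quest goal actor, judging by its name the base for specific goal classes.
; On begin play it passes its questions and itself to its sub-goal info widget.
; Player radius events toggle that widget, showing it only if the actor's class matches a sub-goal in the player's current quests.
; A valid interaction records the class on the character, notifies the quest manager and destroys the actor.
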(event EventOnInteractwith
  (params (Character :type Motion%20Controller%20Pawn%20Object%20Reference))
  (bind _self self)
  (bind _questmanagerref (Variables|/Game/VirtualRealityBP/Blueprints/MotionControllerPawn.MotionControllerPawn_C|GetQuestManagerRef Character))
  (bind _returnvalue (Utilities|GetClass _self))
  ;[1 1 1] Interact with
  (bind _out (CallFunction|GoalforCurrentQuest _questmanagerref))
  (if _out
    (Utilities|Array|Add (Variables|/Game/VirtualRealityBP/Blueprints/MotionControllerPawn.MotionControllerPawn_C|GetAllGoalsInteract Character) _returnvalue)
    (Default|OnInteractGoal _questmanagerref _returnvalue)
    (Actor|DestroyActor)
    (Variables|Default|SetAnyInteraction? true)))

(event EventBeginPlay
  (bind _asw_sub_goal_info (Utilities|Casting|CastTow_SubGoalInfo (UserInterface|GetUserWidgetObject (Variables|Default|GetWidget))))
  (Variables|/Game/Widgets/w_SubGoalInfo.w_SubGoalInfo_C|SetQuestionsArray _asw_sub_goal_info (Variables|Default|GetQuestionsArray))
  (Variables|/Game/Widgets/w_SubGoalInfo.w_SubGoalInfo_C|SetBP_SubGoal _asw_sub_goal_info self))

(event EventOnEnterPlayerRadius
  (params (Character :type Motion%20Controller%20Pawn%20Object%20Reference))
  (bind _widget (Variables|Default|GetWidget))
  ;[1 1 1] Enter radius
  (bind _asw_sub_goal_info (Utilities|Casting|CastTow_SubGoalInfo (UserInterface|GetUserWidgetObject _widget)))
  (Variables|/Game/Widgets/w_SubGoalInfo.w_SubGoalInfo_C|SetCharacter _asw_sub_goal_info Character)
  (bind _out (CallFunction|GoalforCurrentQuest (Variables|/Game/VirtualRealityBP/Blueprints/MotionControllerPawn.MotionControllerPawn_C|GetQuestManagerRef Character)))
  (if _out
    (if (not (Variables|Default|GetAnyInteraction?))
      (Rendering|SetVisibility _widget true false))))

(event EventOnLeavePlayerRadius
  (params (Character :type Motion%20Controller%20Pawn%20Object%20Reference))
  ;[1 1 1] Leave radius
  (Rendering|SetVisibility (Variables|Default|GetWidget) false false))

(fn ConstructionScript)

(fn GoalforCurrentQuest
  (params (QuestManager :type BP%20Quest%20Manager%20Object%20Reference))
  (bind _array_element (Utilities|Array|ForEachLoopwithBreak (Variables|/Game/Blueprints/QuestsManager/BP_QuestManager.BP_QuestManager_C|GetCurrentQuestActors QuestManager) :!label _label)
    (:LoopBody
      (bind _array_element_2 (Utilities|Array|ForEachLoopwithBreak (.SubGoals (Utilities|Struct|Breaks_QuestInfo (Variables|/Game/Blueprints/Quests/BP_MasterQuest.BP_MasterQuest_C|GetQuestInfo _array_element))))
        (:LoopBody
          (if (== (.GoalClass (Utilities|Struct|Breaks_GoalInfo _array_element_2)) (Utilities|GetClass self))
            (LocalVariables|SetGoalForCurrentQuest? true)
            (goto _label Break)))))
    (:Completed
      (return (LocalVariables|GetGoalForCurrentQuest?)))))