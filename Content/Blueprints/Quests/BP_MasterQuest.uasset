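; Master quest actor that tracks a quest's sub-goals and moves the game to the next level when they are all completed.
; Setup activates each QuestInfo sub-goal and adds a widget for it to the main UI; completion removes both.
; Clearing the last goal flags success, stops the pawn's timer and fades out.
; It then opens a random, non-repeating level from the GameInstance map with its quest class, or l_end once three or fewer remain.
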(event Custom|EndQuest
  (bind _asmotion_controller_pawn (Utilities|Casting|CastToMotionControllerPawn (Game|Player|GetPlayerPawn 0))
    (:then
      (Audio|Components|Audio|Stop (Variables|/Game/VirtualRealityBP/Blueprints/MotionControllerPawn.MotionControllerPawn_C|GetTimerSubGoal _asmotion_controller_pawn)))
    (:CastFailed
      _))
  (Utilities|FlowControl|Delay 2.5)
  (CameraFades|StartCameraFade :self (Game|GetPlayerCameraManager 0) :ToAlpha 1.0 :Duration 1.0 :bHoldWhenFinished true)
  (Utilities|FlowControl|Delay 2.0)
  (bind _asbp_game_instance (Utilities|Casting|CastToBP_GameInstance (Game|GetGameInstance)))
  (if (> (Utilities|Map|Length (Variables|/Game/Blueprints/BP_GameInstance.BP_GameInstance_C|GetLevelStructure _asbp_game_instance)) 3)
    (bind _keys (Utilities|Map|Keys (Variables|/Game/Blueprints/BP_GameInstance.BP_GameInstance_C|GetLevelStructure _asbp_game_instance)))
    (Variables|Default|SetQuestIndex (Math|Random|RandomIntegerinRange 0 (- (Utilities|Map|Length (Variables|/Game/Blueprints/BP_GameInstance.BP_GameInstance_C|GetLevelStructure _asbp_game_instance)) 1)))
    (Variables|Default|SetLevelName (Utilities|Array|Get(acopy) _keys (Variables|Default|GetQuestIndex)))
    (Variables|/Game/Blueprints/BP_GameInstance.BP_GameInstance_C|SetQuestClass _asbp_game_instance (.Value (Utilities|Map|Find (Variables|/Game/Blueprints/BP_GameInstance.BP_GameInstance_C|GetLevelStructure _asbp_game_instance) (Variables|Default|GetLevelName))))
    (Utilities|Map|Remove (Variables|/Game/Blueprints/BP_GameInstance.BP_GameInstance_C|GetLevelStructure _asbp_game_instance) (Variables|Default|GetLevelName))
    (Variables|/Game/Blueprints/BP_GameInstance.BP_GameInstance_C|SetLevelStructure _asbp_game_instance (Variables|/Game/Blueprints/BP_GameInstance.BP_GameInstance_C|GetLevelStructure _asbp_game_instance))
    (Game|OpenLevel(byName) (Variables|Default|GetLevelName))
    (else
      (Game|OpenLevel(byName) "l_end"))))

(event EventBeginPlay)

(event Collision|EventActorBeginOverlap
  (params (OtherActor :type Actor%20Object%20Reference)))

(event EventTick
  (params (DeltaSeconds :type Float%20%28single-precision%29)))

(fn ConstructionScript)

(fn CompleteSubGoals
  (params (SubGoalIndex :type Integer))
  (bind _questinfo (Variables|QuestInfo|GetQuestInfo))
  (bind _subgoals (Utilities|Struct|Breaks_QuestInfo _questinfo))
  (LocalVariables|SetLocalGoalIndex SubGoalIndex)
  (if (Utilities|Array|ContainsItem (Variables|Default|GetCurrentGoalIndicies) (LocalVariables|GetLocalGoalIndex))
    (bind _output_get (LocalVariables|SetLocalCompletedGoal (Utilities|Array|Get(acopy) _subgoals (LocalVariables|GetLocalGoalIndex))))
    (Utilities|Array|RemoveItem (Variables|Default|GetCurrentGoal) (LocalVariables|GetLocalCompletedGoal))
    (LocalVariables|SetLocalWidgetIndex (Utilities|Array|FindItem _subgoals _output_get))
    (Utilities|Array|RemoveItem (Variables|Default|GetCurrentGoalIndicies) (LocalVariables|GetLocalGoalIndex))
    (CallFunction|UpdateSubGoals)
    (Widget|RemovefromParent (Utilities|Array|Get(acopy) (Variables|/Game/Widgets/w_MainWidget.w_MainWidget_C|GetSubGoals (Variables|Default|GetMainWidget)) (LocalVariables|GetLocalWidgetIndex)))
    (if (<= (Utilities|Array|Length (Variables|Default|GetCurrentGoal)) 0)
      (bind _asbp_game_instance (Utilities|Casting|CastToBP_GameInstance (Game|GetGameInstance)))
      (Variables|/Game/Blueprints/BP_GameInstance.BP_GameInstance_C|SetFirstQuest? _asbp_game_instance false)
      (Variables|/Game/Blueprints/BP_GameInstance.BP_GameInstance_C|SetQuestSuccess? _asbp_game_instance true)
      (CallFunction|EndQuest))
    (else
      (return false))))

(fn GoalatIndex
  (params (Index :type Integer))
  (return (Utilities|Array|Get(acopy) (.SubGoals (Utilities|Struct|Breaks_QuestInfo (Variables|QuestInfo|GetQuestInfo))) Index)))

(fn UpdateSubGoals
  (Utilities|Array|Clear (Variables|Default|GetCurrentGoal))
  (for _array_element (Variables|Default|GetCurrentGoalIndicies)
    (Utilities|Array|Add (Variables|Default|GetCurrentGoal) (Utilities|Array|Get(acopy) (.SubGoals (Utilities|Struct|Breaks_QuestInfo (Variables|QuestInfo|GetQuestInfo))) _array_element)))
  (return))

(fn SetupStartingGoals
  (Utilities|Array|Clear (Variables|Default|GetCurrentGoalIndicies))
  (for (_ _array_index) (.SubGoals (Utilities|Struct|Breaks_QuestInfo (Variables|QuestInfo|GetQuestInfo)))
    (Utilities|Array|Add (Variables|Default|GetStartingSubGoalIndices) _array_index))
  (for _array_element (Variables|Default|GetStartingSubGoalIndices)
    (CallFunction|AddGoalforIndex _array_element)))

(fn AddGoalforIndex
  (params (Index :type Integer))
  (bind _mainwidget (Variables|Default|GetMainWidget))
  (bind _output_get (LocalVariables|SetLocalIndex Index))
  (if (CallFunction|GoalFound? _output_get)
    (Utilities|Array|Add (Variables|Default|GetCurrentGoalIndicies) (LocalVariables|GetLocalIndex))
    (Utilities|Array|Add (Variables|Default|GetCurrentGoal) (CallFunction|GoalatIndex (LocalVariables|GetLocalIndex)))
    (bind _returnvalue (UserInterface|CreateWidget "/Game/Widgets/w_SubGoals.w_SubGoals_C" 0 (CallFunction|GoalatIndex (LocalVariables|GetLocalIndex))))
    (Widget|Panel|AddChild (Variables|/Game/Widgets/w_MainWidget.w_MainWidget_C|GetQuestList _mainwidget) _returnvalue)
    (Utilities|Array|Add (Variables|/Game/Widgets/w_MainWidget.w_MainWidget_C|GetSubGoals _mainwidget) _returnvalue)
    (return)))

(fn GoalFound?
  (params (Index :type Integer))
  (return (< Index (Utilities|Array|Length (.SubGoals (Utilities|Struct|Breaks_QuestInfo (Variables|QuestInfo|GetQuestInfo)))))))